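; Environmental nebula hazard that deals damage over time to ships inside its capsule volume.
; Each tick it iterates the capsule's overlapping components, casts their owners to ShipBase and applies frame-time-scaled damage.
; NebulaType routes that damage to the ship's shield, hull, room or crew component, with room and crew passed an empty target.
; Damage applies per overlapping component, so a ship with several can take multiple hits per tick.
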(event EventTick
  (params (DeltaSeconds :type Float%20%28single-precision%29))
  (bind _nebuladamagepersecond (Variables|NebulaStats|GetNebulaDamagePerSecond))
  (bind _returnvalue (* _nebuladamagepersecond DeltaSeconds))
  (for _array_element (Class|PrimitiveComponent|GetOverlappingComponents (Variables|Default|GetCapsule))
    (bind _asship_base (Utilities|Casting|CastToShipBase (Components|GetOwner _array_element)))
    (switch Utilities|FlowControl|Switch|SwitchonNebulaDamageType (Variables|NebulaStats|GetNebulaType)
      (:NewEnumerator0
        (Default|DamageOverTime (Variables|/Game/Assets/Blueprints/PlayableShips/Base_Ship/ShipBase.ShipBase_C|GetShieldComponent _asship_base) _returnvalue))
      (:NewEnumerator1
        (Default|DamageOverTime (Variables|/Game/Assets/Blueprints/PlayableShips/Base_Ship/ShipBase.ShipBase_C|GetHullComponent _asship_base) _returnvalue))
      (:NewEnumerator2
        (Default|DamageOverTime (Variables|/Game/Assets/Blueprints/PlayableShips/Base_Ship/ShipBase.ShipBase_C|GetRoomComponent _asship_base) _returnvalue))
      (:NewEnumerator3
        (Default|DamageOverTime (Variables|/Game/Assets/Blueprints/PlayableShips/Base_Ship/ShipBase.ShipBase_C|GetCrewComponent _asship_base) _returnvalue)))))

(fn ConstructionScript)