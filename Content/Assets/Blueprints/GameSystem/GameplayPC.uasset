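; Player controller for a spaceship game that creates the gameplay HUD, toggles the mouse cursor and lets chat-style viewers act as crew.
; The WarpCharge axis drives impulse lockout, warp movement, FOV and tunnel effect, with a velocity-scaled sphere trace for impact warnings.
; Viewer messages are parsed into character creation through HeraldGameMode or orders to the ship's CrewComponent.
; Clicks line-trace from the cursor to set the selected weapon's target.
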(event Custom|ViewerCommand
  (params (User :type String) (Message :type String))
  (bind _returnvalue (Game|GetGameMode))
  (bind _asherald_game_mode (Utilities|Casting|CastToHeraldGameMode _returnvalue))
  (bind _character (CallFunction|GetCharacterName User))
  (bind _found_ (CallFunction|CrewFound? _character))
  (if _found_
    (bind (_outcommand _outparameters) (CallFunction|SplitCommandString Message :!label _label))
    (if _found_
      (CallFunction|IssueViewerCommand User _character _outcommand _outparameters :!label _label_2)
      (elif (Utilities|Enum|Equal(Enum) _outcommand "board")
        (goto _label_2)))
    (else
      (bind _keys (Utilities|Map|Keys (Variables|/Game/Assets/Blueprints/GameSystem/HeraldGameMode.HeraldGameMode_C|GetCharNameToViewerName _asherald_game_mode)))
      (if (Utilities|Array|ContainsItem _keys _character)
        (goto _label)
        (else
          (bind (_outcommand_2 _outparameters_2) (CallFunction|SplitCommandString Message))
          (if (Utilities|Enum|Equal(Enum) _outcommand_2 "start")
            (Default|CreateCrew _asherald_game_mode (Utilities|String|JoinStringArray _outparameters_2 "") 0 User)))))))

(event Custom|Click
  (bind (_worldlocation _worlddirection) (Game|Player|ConvertMouseLocationToWorldSpace))
  (bind _returnvalue (Game|GetPlayerCharacter 0))
  (bind _returnvalue_2 (* _worlddirection 1e+02))
  (bind _asship_base (Utilities|Casting|CastToShipBase _returnvalue))
  (bind _returnvalue_3 (+ _worldlocation _returnvalue_2))
  (bind _weaponscomponent (Variables|/Game/Assets/Blueprints/PlayableShips/Base_Ship/ShipBase.ShipBase_C|GetWeaponsComponent _asship_base))
  (bind _selectedweapon (Variables|/Game/Assets/Blueprints/PlayableShips/ShipComponents/WeaponsComponent/WeaponsComponent.WeaponsComponent_C|GetSelectedWeapon _weaponscomponent))
  (bind (_outhit _returnvalue_4) (Collision|LineTraceByChannel _returnvalue_3 (+ _returnvalue_3 (* (- _returnvalue_3 (Transformation|GetActorLocation (Game|GetPlayerCameraManager 0))) 4e+03)) "TraceTypeQuery1" false 0 "None"))
  (bind _asship_base_2 (Utilities|Casting|CastToShipBase (Game|GetPlayerCharacter 0)))
  (if (!= _asship_base_2 (.HitActor (Collision|BreakHitResult _outhit)))
    (if (and (> _selectedweapon 0) _returnvalue_4)
      (bind _values (Utilities|Map|Values (Variables|/Game/Assets/Blueprints/PlayableShips/ShipComponents/WeaponsComponent/WeaponsComponent.WeaponsComponent_C|GetWeaponMounts _weaponscomponent)))
      (if (<= _selectedweapon (Utilities|Array|Length _values))
        (Variables|/Game/Assets/Blueprints/PlayableShips/ShipComponents/WeaponsComponent/WeaponObject.WeaponObject_C|SetTargetActor (Variables|/Game/Assets/Blueprints/PlayableShips/ShipComponents/WeaponsComponent/Mount.Mount_C|GetWeaponInstance (Utilities|Array|Get(acopy) _values (- _selectedweapon 1))) (.HitActor (Collision|BreakHitResult _outhit)))))))

(event Custom|IssueViewerCommand
  (params (Viewer :type String) (Character :type String) (Command :type String) (Parameters :type Array%20of%20Strings))
  (bind _returnvalue (Game|GetPlayerCharacter 0))
  (bind _output (Utilities|Array|Get(acopy) Parameters))
  (bind _asship_base (Utilities|Casting|CastToShipBase _returnvalue))
  (bind _crewcomponent (Variables|/Game/Assets/Blueprints/PlayableShips/Base_Ship/ShipBase.ShipBase_C|GetCrewComponent _asship_base))
  (switch string Command
    (:Board
      (Default|Board _crewcomponent Character _output))
    (:Repair
      (Default|RepairCommand _crewcomponent Character))
    (:Calibrate
      (Default|CalibrateCommand _crewcomponent Character "" 1.0))
    (:Move
      (Default|Move _crewcomponent Character _output))
    (:Away
      (Default|AssignAwayCrew _crewcomponent Character))))

(event EventBeginPlay
  (bind _returnvalue (UserInterface|CreateWidget "/Game/Assets/Widgets/GameplayHUD.GameplayHUD_C"))
  (bind _output_get (Variables|Default|SetGameplayHUD _returnvalue))
  (UserInterface|Viewport|AddtoViewport _output_get 0)
  (Input|SetInputModeGameandUI self _output_get "DoNotLock" false))

(event EventTick
  (params (DeltaSeconds :type Float%20%28single-precision%29))
  (bind (_sizex _sizey) (HUD|GetViewportSize))
  (bind _asgameplay_pc (Utilities|Casting|CastToGameplayPC (Game|GetPlayerController 0)))
  (if (not (Variables|GameplayPC_C|GetCursorShown? _asgameplay_pc))
    (Class|PlayerController|SetMouseLocation (/ _sizex 2) (/ _sizey 2))))

(event Input|AxisEvents|InputAxisWarpCharge
  (params (AxisValue :type Float%20%28single-precision%29))
  (bind _returnvalue (Utilities|Time|GetWorldDeltaSeconds))
  (bind _controlledship (Variables|Default|GetControlledShip))
  (bind _gameplayhud (Variables|Default|GetGameplayHUD))
  (bind _controlledship_2 (Variables|Default|GetControlledShip))
  (bind _mesh (Variables|/Script/Engine.Character|GetMesh _controlledship))
  (bind _followcamera (Variables|/Game/Assets/Blueprints/PlayableShips/Base_Ship/ShipBase.ShipBase_C|GetFollowCamera _controlledship_2))
  (bind _mesh_2 (Variables|/Script/Engine.Character|GetMesh _controlledship))
  (bind _returnvalue_2 (Transformation|GetWorldLocation _mesh))
  (bind _returnvalue_3 (Math|Vector|GetRightVector _mesh_2))
  (bind _asship_base (Utilities|Casting|CastToShipBase _controlledship))
  (if (> AxisValue 0.0)
    (bind _output_get (Variables|/Game/Assets/Blueprints/PlayableShips/ShipComponents/ImpulseComponent/ImpulseComponent.ImpulseComponent_C|SetWarpCharge (Variables|/Game/Assets/Blueprints/PlayableShips/Base_Ship/ShipBase.ShipBase_C|GetImpulseComponent _asship_base) (Math|Float|Clamp(Float) (+ (Variables|/Game/Assets/Blueprints/PlayableShips/ShipComponents/ImpulseComponent/ImpulseComponent.ImpulseComponent_C|GetWarpCharge (Variables|/Game/Assets/Blueprints/PlayableShips/Base_Ship/ShipBase.ShipBase_C|GetImpulseComponent _asship_base)) (* (* AxisValue _returnvalue) 0.2)))))
    (else
      (Variables|/Game/Assets/Blueprints/PlayableShips/ShipComponents/ImpulseComponent/ImpulseComponent.ImpulseComponent_C|SetWarpCharge (Variables|/Game/Assets/Blueprints/PlayableShips/Base_Ship/ShipBase.ShipBase_C|GetImpulseComponent _asship_base) (Math|Float|Clamp(Float) (- (Variables|/Game/Assets/Blueprints/PlayableShips/ShipComponents/ImpulseComponent/ImpulseComponent.ImpulseComponent_C|GetWarpCharge (Variables|/Game/Assets/Blueprints/PlayableShips/Base_Ship/ShipBase.ShipBase_C|GetImpulseComponent _asship_base)) (* _returnvalue 1.0))))))
  (if (> (Variables|/Game/Assets/Blueprints/PlayableShips/ShipComponents/ImpulseComponent/ImpulseComponent.ImpulseComponent_C|GetWarpCharge (Variables|/Game/Assets/Blueprints/PlayableShips/Base_Ship/ShipBase.ShipBase_C|GetImpulseComponent _asship_base)) 0.0)
    (Variables|/Game/Assets/Blueprints/PlayableShips/ShipComponents/BaseComponent/BaseShipComponent.BaseShipComponent_C|SetDisabled? (Variables|/Game/Assets/Blueprints/PlayableShips/Base_Ship/ShipBase.ShipBase_C|GetImpulseComponent _asship_base) true)
    (if (> (Variables|/Game/Assets/Blueprints/PlayableShips/ShipComponents/ImpulseComponent/ImpulseComponent.ImpulseComponent_C|GetWarpCharge (Variables|/Game/Assets/Blueprints/PlayableShips/Base_Ship/ShipBase.ShipBase_C|GetImpulseComponent _asship_base)) 0.9)
      (Utilities|IsValid (Variables|Default|GetWarpEffect)
        (:Is%20Valid
          (Camera|SetFieldOfView _followcamera (Math|Float|Max(Float) (* (Variables|/Game/Assets/Blueprints/PlayableShips/ShipComponents/ImpulseComponent/ImpulseComponent.ImpulseComponent_C|GetWarpCharge (Variables|/Game/Assets/Blueprints/PlayableShips/Base_Ship/ShipBase.ShipBase_C|GetImpulseComponent _asship_base)) 1.2e+02) 9e+01)))
        (:Is%20Not%20Valid
          (bind _returnvalue_4 (Effects|SpawnEmitterAttached "/Game/Assets/ParticleSystems/WarpTunnel.WarpTunnel" (Variables|/Script/Engine.Character|GetCapsuleComponent _controlledship_2) "None" "-10000.000000,0.000000,0.000000" "90.000000,0.000000,0.000000" "SnapToTarget"))
          (Variables|Default|SetWarpEffect _returnvalue_4)))
      (Variables|/Script/Engine.CharacterMovementComponent|SetMaxFlySpeed (Variables|/Script/Engine.Character|GetCharacterMovement _asship_base) 1e+09)
      (Variables|/Script/Engine.CharacterMovementComponent|SetMaxAcceleration (Variables|/Script/Engine.Character|GetCharacterMovement _asship_base) 2e+05)
      (Variables|/Script/Engine.CharacterMovementComponent|SetBrakingDecelerationFlying (Variables|/Script/Engine.Character|GetCharacterMovement _asship_base) (* _output_get 1e+09))
      (Pawn|Input|AddMovementInput _asship_base (* (* _returnvalue_3 -1.0) (* (* (Variables|/Game/Assets/Blueprints/PlayableShips/ShipComponents/ImpulseComponent/ImpulseComponent.ImpulseComponent_C|GetWarpMaxSpeed (Variables|/Game/Assets/Blueprints/PlayableShips/Base_Ship/ShipBase.ShipBase_C|GetImpulseComponent _asship_base)) (Utilities|Time|GetWorldDeltaSeconds)) _output_get)) 1.0 false)
      (bind _outactors (Actor|GetAllActorsOfClass "/Game/Assets/Blueprints/PlayableShips/Base_Ship/ShipBase.ShipBase_C"))
      (bind (_outhit _returnvalue_5) (Collision|SphereTraceByChannel _returnvalue_2 (+ _returnvalue_2 (* (* _returnvalue_3 (* (Math|Vector|VectorLength (Variables|/Script/Engine.MovementComponent|GetVelocity (Variables|/Script/Engine.Character|GetCharacterMovement _asship_base))) 1e+01)) -1.0)) 1e+02 "TraceTypeQuery1" false _outactors "None" true "(R=1.000000,G=0.000000,B=0.000000,A=1.000000)" "(R=0.000000,G=1.000000,B=0.000000,A=1.000000)" 1.0))
      (if (and _returnvalue_5 (!= (Utilities|GetClass (.HitActor (Collision|BreakHitResult _outhit))) "/Game/Assets/Blueprints/Projectiles/BaseProjectile.BaseProjectile_C"))
        (Default|ToggleImpactWarning _gameplayhud true)
        (else
          (Default|ToggleImpactWarning _gameplayhud false)))
      (else
        (Camera|SetFieldOfView _followcamera (Math|Float|Max(Float) (* (Variables|/Game/Assets/Blueprints/PlayableShips/ShipComponents/ImpulseComponent/ImpulseComponent.ImpulseComponent_C|GetWarpCharge (Variables|/Game/Assets/Blueprints/PlayableShips/Base_Ship/ShipBase.ShipBase_C|GetImpulseComponent _asship_base)) 1.2e+02) 9e+01))
        (Utilities|IsValid (Variables|Default|GetWarpEffect)
          (:Is%20Valid
            (Components|Activation|Deactivate (Variables|Default|GetWarpEffect))
            (Default|ToggleImpactWarning (Variables|Default|GetGameplayHUD) false))
          (:Is%20Not%20Valid
            (Variables|/Script/Engine.CharacterMovementComponent|SetMaxFlySpeed (Variables|/Script/Engine.Character|GetCharacterMovement _asship_base) 1e+03 :!label _label)
            (Variables|/Script/Engine.CharacterMovementComponent|SetMaxAcceleration (Variables|/Script/Engine.Character|GetCharacterMovement _asship_base) 5e+02)
            (Variables|/Script/Engine.CharacterMovementComponent|SetBrakingDecelerationFlying (Variables|/Script/Engine.Character|GetCharacterMovement _asship_base) 0.0)))))
    (else
      (Variables|/Game/Assets/Blueprints/PlayableShips/ShipComponents/BaseComponent/BaseShipComponent.BaseShipComponent_C|SetDisabled? (Variables|/Game/Assets/Blueprints/PlayableShips/Base_Ship/ShipBase.ShipBase_C|GetImpulseComponent _asship_base) false)
      (goto _label))))

(event Input|KeyboardEvents|T
  (params (Key :type Key%20Structure))
  ;[1 1 1] T to type
  (:Pressed
    (if (Variables|Default|GetCursorShown?)
      (Variables|Default|SetCursorShown? false)
      (Variables|Default|SetbShowMouseCursor false)
      (else
        (Variables|Default|SetCursorShown? true)
        (Variables|Default|SetbShowMouseCursor true)))))

(fn ConstructionScript)

(fn SplitCommandString
  (params (Command :type String))
  (for (_array_element _array_index) (Utilities|String|ParseIntoArray Command " ")
    (if (> _array_index 0)
      (Utilities|Array|Add (LocalVariables|GetTempCommands) (Utilities|String|ToLower _array_element))
      (else
        (LocalVariables|SetTempCommand (Utilities|String|ToLower _array_element)))))
  (return (LocalVariables|GetTempCommand) (LocalVariables|GetTempCommands)))

(fn GetCharacterName
  (params (User :type String))
  (bind _returnvalue (Game|GetGameMode))
  (bind _asherald_game_mode (Utilities|Casting|CastToHeraldGameMode _returnvalue))
  (bind _charnametoviewername (Variables|/Game/Assets/Blueprints/GameSystem/HeraldGameMode.HeraldGameMode_C|GetCharNameToViewerName _asherald_game_mode))
  (bind _values (Utilities|Map|Values _charnametoviewername))
  (for (_array_element _array_index) _values
    (if (Utilities|Enum|Equal(Enum) _array_element User)
      (bind _keys (Utilities|Map|Keys _charnametoviewername))
      (return (Utilities|Array|Get(acopy) _keys _array_index)))))

(fn CrewFound?
  (params (CharacterName :type String))
  (bind _keys (Utilities|Map|Keys (Variables|/Game/Assets/Blueprints/PlayableShips/ShipComponents/CrewComponent/CrewComponent.CrewComponent_C|GetCrew (Variables|/Game/Assets/Blueprints/PlayableShips/Base_Ship/ShipBase.ShipBase_C|GetCrewComponent (Variables|Default|GetControlledShip)))))
  (return (Utilities|Array|ContainsItem _keys (Utilities|String|StringToName CharacterName))))