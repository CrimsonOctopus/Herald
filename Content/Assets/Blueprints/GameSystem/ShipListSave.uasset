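; ShipListSave is a save game object that stores a list of ship names and the controlled ship.
; Its Save event copies both values in through SetData, then writes the object itself to its save slot.
; SetSlotData sets the slot name and user index that Save uses.
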(event Custom|Save
  (params (ShipNames :type Array%20of%20Strings) (ControlledShip :type String))
  (CallFunction|SetData ShipNames ControlledShip)
  (SaveGame|SaveGametoSlot self (Variables|Default|GetSaveSlotName) (Variables|Default|GetUserIndex)))

(fn SetData
  (params (ShipNames :type Array%20of%20Strings) (ControlledShip :type String))
  (Variables|Default|SetShipNames ShipNames)
  (Variables|Default|SetControlledShip ControlledShip))

(fn SetSlotData
  (params (Name :type String) (Index :type Integer))
  (Variables|Default|SetSaveSlotName Name)
  (Variables|Default|SetUserIndex Index))