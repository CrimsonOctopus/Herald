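; Game mode that boots a session from saved ship and viewer-crew lists and keeps registries of both.
; On BeginPlay it spawns ships near the first station, possessing the controlled one, running others as behavior-tree AI, and adding an extra ship if under two.
; Each crew member loads from a save slot named after its viewer and maps to that username.
; Save events write ship names, viewer names and per-crew data through SaveGame objects.
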(event Custom|LoadCrewList
  ;[1 1 1] Load viewer names from file
  (bind _returnvalue (SaveGame|LoadGamefromSlot (Variables|CrewPersistence|GetCrewSaveSlotName) (Variables|CrewPersistence|GetCrewSaveUserIndex)))
  (if (.bSuccess (Utilities|Casting|CastToCrewListSave _returnvalue))
    (Variables|CrewPersistence|SetCrewListSave (.AsCrew%20List%20Save (Utilities|Casting|CastToCrewListSave _returnvalue)))
    (CallFunction|LoadCrew (Variables|/Game/Assets/Blueprints/PlayableShips/ShipComponents/CrewComponent/CrewListSave.CrewListSave_C|GetUsers (.AsCrew%20List%20Save (Utilities|Casting|CastToCrewListSave _returnvalue))))
    (else
      (Development|PrintString "No ShipList Save")
      (CallFunction|LoadCrew (Utilities|Array|MakeArray)))))

(event Custom|Spawn
  (bind _shiplistsave (Variables|ShipPersistence|GetShipListSave))
  (Utilities|IsValid _shiplistsave
    (:Is%20Valid
      (CallFunction|SpawnShips (Variables|/Game/Assets/Blueprints/GameSystem/ShipListSave.ShipListSave_C|GetShipNames _shiplistsave) (Variables|/Game/Assets/Blueprints/GameSystem/ShipListSave.ShipListSave_C|GetControlledShip _shiplistsave)))
    (:Is%20Not%20Valid
      (CallFunction|SpawnShips (Utilities|Array|MakeArray "")))))

(event Custom|SaveCrewList
  ;[1 1 1] Save the names of all the unique viewers
  (Utilities|IsValid (Variables|CrewPersistence|GetCrewListSave)
    (:Is%20Valid
      _)
    (:Is%20Not%20Valid
      (bind _returnvalue (SaveGame|CreateSaveGameObject "/Game/Assets/Blueprints/PlayableShips/ShipComponents/CrewComponent/CrewListSave.CrewListSave_C"))
      (Variables|CrewPersistence|SetCrewListSave _returnvalue)))
  (bind _values (Utilities|Map|Values (Variables|CrewPersistence|GetCharNameToViewerName)))
  (Default|Save (Variables|CrewPersistence|GetCrewListSave) _values)
  (bind _values_2 (Utilities|Map|Values (Variables|CrewPersistence|GetCharacterNameToCrew)))
  (for _array_element _values_2
    (Utilities|IsValid (Variables|/Game/Assets/Blueprints/PlayableShips/ShipComponents/CrewComponent/CrewObject.CrewObject_C|GetCrewSave _array_element)
      (:Is%20Valid
        (Default|Save (Variables|/Game/Assets/Blueprints/PlayableShips/ShipComponents/CrewComponent/CrewObject.CrewObject_C|GetCrewSave _array_element) _array_element (.Value (Utilities|Map|Find (Variables|CrewPersistence|GetCharNameToViewerName) (Variables|/Game/Assets/Blueprints/PlayableShips/ShipComponents/CrewComponent/CrewObject.CrewObject_C|GetCrewName _array_element))))))))

(event Custom|CreateCrew
  (params (CharacterName :type String) (Save :type Crew%20Member%20Save%20Object%20Reference) (Username :type String))
  (bind _returnvalue (Game|ConstructObjectfromClass "/Game/Assets/Blueprints/PlayableShips/ShipComponents/CrewComponent/CrewObject.CrewObject_C" self))
  (Utilities|IsValid Save
    (:Is%20Valid
      (bind _output_get (Variables|/Game/Assets/Blueprints/PlayableShips/ShipComponents/CrewComponent/CrewObject.CrewObject_C|SetCrewSave _returnvalue Save))
      (Default|Initialize _returnvalue _output_get (Variables|ShipPersistence|GetControlledShip)))
    (:Is%20Not%20Valid
      (bind _returnvalue_2 (SaveGame|CreateSaveGameObject "/Game/Assets/Blueprints/PlayableShips/ShipComponents/CrewComponent/CrewMemberSave.CrewMemberSave_C"))
      (bind _output_get_2 (Variables|/Game/Assets/Blueprints/PlayableShips/ShipComponents/CrewComponent/CrewObject.CrewObject_C|SetCrewSave _returnvalue _returnvalue_2))
      (Variables|/Game/Assets/Blueprints/PlayableShips/ShipComponents/CrewComponent/CrewMemberSave.CrewMemberSave_C|SetCrewName _output_get_2 (Utilities|String|StringToName CharacterName))
      (Default|Initialize _returnvalue _output_get_2 (Variables|ShipPersistence|GetControlledShip))))
  (Utilities|Map|Add (Variables|CrewPersistence|GetCharacterNameToCrew) CharacterName _returnvalue)
  (Utilities|Map|Add (Variables|CrewPersistence|GetCharNameToViewerName) CharacterName Username))

(event Custom|SpawnAIShip
  (params (Location\ :type Vector))
  (bind _returnvalue (Game|GetGameMode))
  (bind _asherald_game_mode (Utilities|Casting|CastToHeraldGameMode _returnvalue))
  (if (< (Utilities|Map|Length (Variables|HeraldGameMode_C|GetShips _asherald_game_mode)) 2)
    (CallFunction|SpawnShip _asherald_game_mode (+ Location\ (* (Math|Random|RandomUnitVector) (Math|Random|RandomFloatinRange 1e+03 5e+03))) "0, 0, 0" false)))

(event Custom|LoadShipList
  ;[1 1 1] Load ship names from file and spawn the ship objects
  (bind _returnvalue (SaveGame|LoadGamefromSlot (Variables|ShipPersistence|GetShipSaveSlotName) (Variables|ShipPersistence|GetShipSaveUserIndex)))
  (if (.bSuccess (Utilities|Casting|CastToShipListSave _returnvalue))
    (Variables|ShipPersistence|SetShipListSave (.AsShip%20List%20Save (Utilities|Casting|CastToShipListSave _returnvalue)))))

(event Custom|SaveShipList
  (params (Controlled :type Ship%20Base%20Object%20Reference))
  ;[1 1 1] Save the names off each ship to file
  (bind _returnvalue (SaveGame|CreateSaveGameObject "/Game/Assets/Blueprints/GameSystem/ShipListSave.ShipListSave_C"))
  (bind _output_get (Variables|ShipPersistence|SetShipListSave _returnvalue))
  (bind _keys (Utilities|Map|Keys (Variables|ShipPersistence|GetShips)))
  (Default|Save _output_get _keys (Variables|/Game/Assets/Blueprints/PlayableShips/Base_Ship/ShipBase.ShipBase_C|GetInstanceName Controlled)))

(event EventBeginPlay
  (CallFunction|LoadShipList)
  (CallFunction|LoadCrewList)
  (Utilities|FlowControl|Delay 0.2)
  (bind _outactors (Actor|GetAllActorsOfClass "/Game/Assets/Blueprints/PlayableShips/Base_Ship/StationBase.StationBase_C"))
  (bind _output_get (Variables|ShipPersistence|SetStartingStation (Utilities|Array|Get(acopy) _outactors)))
  (CallFunction|Spawn)
  (CallFunction|SpawnAIShip (Transformation|GetActorLocation _output_get)))

(fn ConstructionScript)

(fn SpawnShips
  (params (Ships :type Array%20of%20Strings) (Controlled :type String))
  (bind _returnvalue (Game|GetPlayerController 0))
  (bind _returnvalue_2 (Game|GetPlayerController 0))
  (bind _returnvalue_3 (Math|Random|RandomUnitVector))
  (bind _startingstation (Variables|ShipPersistence|GetStartingStation))
  (bind _returnvalue_4 (Transformation|GetActorLocation _startingstation))
  (bind _returnvalue_5 (* _returnvalue_3 1e+02))
  (bind _returnvalue_6 (+ _returnvalue_4 _returnvalue_5))
  (bind _returnvalue_7 (Math|Transform|MakeTransform _returnvalue_6))
  (if (or (or (<= (Utilities|Array|Length Ships) 0) (Utilities|Enum|Equal(Enum) Controlled "")) (not (Utilities|Array|ContainsItem Ships Controlled)))
    ;[1 1 1] If no controlled ship or list is empty, spawn player and set it to controlled ship
    (bind _returnvalue_8 (Game|SpawnActorfromClass "/Game/Assets/Blueprints/PlayableShips/Base_Ship/ShipBase.ShipBase_C" _returnvalue_7 "AlwaysSpawn" 0 0))
    (Pawn|Possess _returnvalue _returnvalue_8)
    (bind _asgameplay_pc (Utilities|Casting|CastToGameplayPC _returnvalue))
    (Default|Initialize _returnvalue_8 "Prototron" false)
    (Variables|/Game/Assets/Blueprints/GameSystem/GameplayPC.GameplayPC_C|SetControlledShip _asgameplay_pc _returnvalue_8)
    (Variables|ShipPersistence|SetControlledShip _returnvalue_8)
    (CallFunction|RegisterShip _returnvalue_8)
    (else
      ;[1 1 1] For each ship, if this ship is the controlled ship, spawn and posses it, otherwise just spawn it
      (for _array_element Ships
        (if (Utilities|Enum|Equal(Enum) _array_element Controlled)
          (bind _returnvalue_9 (Game|SpawnActorfromClass "/Game/Assets/Blueprints/PlayableShips/Base_Ship/ShipBase.ShipBase_C" _returnvalue_7 "AlwaysSpawn" 0 0))
          (Pawn|Possess _returnvalue_2 _returnvalue_9)
          (bind _asgameplay_pc_2 (Utilities|Casting|CastToGameplayPC _returnvalue_2))
          (Variables|/Game/Assets/Blueprints/GameSystem/GameplayPC.GameplayPC_C|SetControlledShip _asgameplay_pc_2 _returnvalue_9)
          (Default|Initialize _returnvalue_9 "Prototron" false)
          (Variables|ShipPersistence|SetControlledShip _returnvalue_9)
          (CallFunction|RegisterShip _returnvalue_9)
          (else
            (bind _returnvalue_10 (AI|SpawnAIFromClass "/Game/Assets/Blueprints/PlayableShips/Base_Ship/ShipBase.ShipBase_C" "/Game/ShipTree.ShipTree" _returnvalue_6 "0, 0, 0" true))
            (bind _asship_base (Utilities|Casting|CastToShipBase _returnvalue_10))
            (Default|Initialize _asship_base "Crusher" false)
            (CallFunction|RegisterShip _asship_base)))))))

(fn RegisterShip
  (params (Ship :type Ship%20Base%20Object%20Reference%20%28by%20ref%29))
  (bind _ships (Variables|ShipPersistence|GetShips))
  (if (Utilities|Enum|Equal(Enum) (Variables|/Game/Assets/Blueprints/PlayableShips/Base_Ship/ShipBase.ShipBase_C|GetInstanceName Ship) "")
    (bind _output_get (Variables|/Game/Assets/Blueprints/PlayableShips/Base_Ship/ShipBase.ShipBase_C|SetInstanceName Ship (Utilities|String|Append (Variables|/Game/Assets/Blueprints/PlayableShips/Base_Ship/ShipBase.ShipBase_C|GetShipName Ship) (Utilities|String|ToString(Integer) (Utilities|Map|Length _ships)))))
    (Utilities|Map|Add _ships _output_get Ship)))

(fn LoadCrew
  (params (UserNames :type Array%20of%20Strings))
  (if (not (<= (Utilities|Array|Length UserNames) 0))
    (for _array_element UserNames
      (bind _returnvalue (SaveGame|LoadGamefromSlot _array_element))
      (CallFunction|CreateCrew (Utilities|String|ToString(Name) (Variables|/Game/Assets/Blueprints/PlayableShips/ShipComponents/CrewComponent/CrewMemberSave.CrewMemberSave_C|GetCrewName (.AsCrew%20Member%20Save (Utilities|Casting|CastToCrewMemberSave _returnvalue)))) (.AsCrew%20Member%20Save (Utilities|Casting|CastToCrewMemberSave _returnvalue)) _array_element))))

(fn GetCharacterPlayer
  (params (User :type String))
  (bind _returnvalue (Game|GetGameMode))
  (bind _asherald_game_mode (Utilities|Casting|CastToHeraldGameMode _returnvalue))
  (bind _charnametoviewername (Variables|HeraldGameMode_C|GetCharNameToViewerName _asherald_game_mode))
  (bind _values (Utilities|Map|Values _charnametoviewername))
  (for (_array_element _array_index) _values
    (if (Utilities|Enum|Equal(Enum) _array_element User)
      (Development|PrintString "Hello")
      (bind _keys (Utilities|Map|Keys _charnametoviewername))
      (return (Utilities|Array|Get(acopy) _keys _array_index)))))

(fn SpawnShip
  (params (Location :type Vector) (Rotation :type Rotator) (Log? :type Boolean))
  (bind _returnvalue (Game|SpawnActorfromClass "/Game/Assets/Blueprints/PlayableShips/Base_Ship/ShipBase.ShipBase_C" (Math|Transform|MakeTransform Location Rotation) "AlwaysSpawn" 0 0))
  (if Log?
    (Development|PrintText (Utilities|Text|FormatText (Utilities|Text|ToText(String) (Utilities|GetDisplayName _returnvalue))) true true "(R=0.000000,G=1.000000,B=0.012258,A=1.000000)" 15.0))
  (Default|Initialize _returnvalue "Crusher" Log?)
  (CallFunction|RegisterShip _returnvalue))