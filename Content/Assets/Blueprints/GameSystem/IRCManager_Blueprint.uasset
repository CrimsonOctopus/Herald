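; IRC manager Blueprint that passes viewer chat messages into gameplay.
; HandleChatMessage registers first-time senders in the ViewerNames list through NewViewer.
; It then strips the first two characters from every message and forwards user and text to ViewerCommand on player 0's GameplayPC controller.
; The chat connection itself is not in this graph, and BeginPlay is empty.
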(event Custom|NewViewer
  (params (ViewerName :type String))
  (Utilities|Set|Add (Variables|Default|GetViewerNames) ViewerName))

(event EventBeginPlay)

(event Collision|EventActorBeginOverlap
  (params (OtherActor :type Actor%20Object%20Reference)))

(event EventTick
  (params (DeltaSeconds :type Float%20%28single-precision%29)))

(event EventHandleChatMessage
  (params (user :type String) (msg :type String))
  (if (Utilities|Set|Contains (Variables|Default|GetViewerNames) user)
    _
    (else
      (CallFunction|NewViewer user)))
  (Default|ViewerCommand (.AsGameplay%20PC (Utilities|Casting|CastToGameplayPC (Game|GetPlayerController 0))) user (Utilities|String|GetSubstring msg 2 (- (Utilities|String|Len msg) 2))))

(fn ConstructionScript)