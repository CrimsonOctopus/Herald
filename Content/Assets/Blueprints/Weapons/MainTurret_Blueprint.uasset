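; Main ship turret weapon that tracks a target, defaulting to player 0's character, and fires projectiles at it.
; WeaponTick acquires the target, yaws around the mount's up vector, then checks cooldown, firing angle and loaded rounds; only the timer's refire checks range.
; Hits are pre-rolled d20-plus-Accuracy and passed to a projectile launched with randomized offset.
; Hit follows estimated travel time but only casts to ShipBase, applying no damage.
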(event Custom|SetTargetActor
  (params (Target :type Actor%20Object%20Reference))
  ;[1 1 1] Set the target actor for this weapon
  (Variables|TurretInfo|SetTargetActor Target))

(event Custom|RotateTowardsTarget
  (bind _targetactor (Variables|TurretInfo|GetTargetActor))
  (bind _mountpoint (Variables|TurretInfo|GetMountPoint))
  (bind _returnvalue (Math|Vector|GetUpVector _mountpoint))
  ;[1 1 1] Rotate the turret along it's axis toward the target
  (Utilities|IsValid _targetactor
    (:Is%20Valid
      (Transformation|SetActorRotation (Math|Rotator|MakeRotfromZX _returnvalue (Math|Vector|Normalize (Math|Vector|ProjectVectorontoPlane (Math|Vector|GetUnitDirection(Vector) (Transformation|GetActorLocation) (Transformation|GetActorLocation _targetactor)) _returnvalue)))))))

(event Custom|WaitUntilHit
  ;[1 1 1] Delay for a number of seconds equal to the the projectile's speed (u/s) divided by the distance to the target
  (Utilities|FlowControl|Delay (/ (Math|Vector|VectorLength (- (Transformation|GetWorldLocation (Variables|Default|GetMuzzle1)) (Transformation|GetActorLocation (Variables|TurretInfo|GetTargetActor)))) (.Speed (Utilities|GetClassDefaults (Variables|TurretInfo|GetProjectile))))))

(event Custom|WeaponTick
  ;[1 1 1] Every tick, rotate the turret and check if we can fire
  (Utilities|IsValid self
    (:Is%20Valid
      (CallFunction|AcquireTarget)
      (CallFunction|RotateTowardsTarget)
      (CallFunction|CheckFire))))

(event Custom|FireProjectile
  ;[1 1 1] If the turret's attack hits, spawn the projectile and set it's target to the enemy, otherwise, set it to a point
  (CallFunction|StartCooldownTimer)
  (bind _hit_ (CallFunction|DidHit?))
  (if _hit_
    (CallFunction|CreateProjectile true)
    (Utilities|FlowControl|Delay (/ (Math|Vector|VectorLength (- (Transformation|GetWorldLocation (Variables|Default|GetMuzzle1)) (Transformation|GetActorLocation (Variables|TurretInfo|GetTargetActor)))) (.Speed (Utilities|GetClassDefaults (Variables|TurretInfo|GetProjectile)))))
    (CallFunction|Hit)
    (else
      (CallFunction|CreateProjectile false)
      (Utilities|FlowControl|Delay (/ (Math|Vector|VectorLength (- (Transformation|GetWorldLocation (Variables|Default|GetMuzzle1)) (Transformation|GetActorLocation (Variables|TurretInfo|GetTargetActor)))) (.Speed (Utilities|GetClassDefaults (Variables|TurretInfo|GetProjectile))))))))

(event Custom|Die
  ;[1 1 1] Destroy the turret if it dies
)

(event Custom|AcquireTarget
  (bind _returnvalue (Game|GetPlayerCharacter 0))
  (if (not (== _returnvalue (Actor|GetParentActor)))
    (Utilities|IsValid _returnvalue
      (:Is%20Valid
        (Utilities|IsValid (Variables|TurretInfo|GetTargetActor)
          (:Is%20Not%20Valid
            (Variables|TurretInfo|SetTargetActor _returnvalue)))))))

(event Custom|CreateProjectile
  (params (Hit? :type Boolean))
  (bind _targetactor (Variables|TurretInfo|GetTargetActor))
  ;[1 1 1] Spawn the projectile and set it's target
  (Game|SpawnActorfromClass (Variables|TurretInfo|GetProjectile) (Transformation|GetWorldTransform (Variables|Default|GetMuzzle1)) "AlwaysSpawn" 0 _targetactor Hit? (Math|Vector|GetUnitDirection(Vector) (Transformation|GetActorLocation) (+ (Transformation|GetActorLocation _targetactor) (+ (* (Transformation|GetActorUpVector _targetactor) (Math|Random|RandomFloatinRange 1e+02 2e+02)) (* (Transformation|GetActorRightVector) (Math|Random|RandomFloatinRange -2e+02 2e+02))))) 0 0))

(event Custom|CheckFire
  ;[1 1 1] If cooldown timer expired and the angle between weapon forward and target <= max fire angle, fire a projectile
  (Utilities|IsValid (Variables|TurretInfo|GetTargetActor)
    (:Is%20Valid
      (if (not (Utilities|Time|IsTimerActivebyHandle (stale Custom|StartCooldownTimer _returnvalue)))
        (if (<= (Class|KismetMathLibrary|DegAcos (Math|Vector|DotProduct (Transformation|GetActorForwardVector) (Math|Vector|Normalize (- (Transformation|GetActorLocation (Variables|TurretInfo|GetTargetActor)) (Transformation|GetActorLocation))))) (Variables|TurretInfo|GetMaxAngle))
          (if (> (Variables|TurretInfo|GetLoadedRounds) 0)
            (CallFunction|FireProjectile)))))))

(event Custom|InitializeWeapon
  (params (Count :type Integer))
  ;[1 1 1] Initialize this weapon's loaded rounds and instance name
  (Variables|TurretInfo|SetLoadedRounds (Variables|TurretInfo|GetMaxRounds))
  (Variables|TurretInfo|SetInstanceName (Utilities|String|ToString(Text) (Utilities|Text|FormatText "{WeaponName}{Count}" (Utilities|Text|ToText(String) (Variables|TurretInfo|GetWeaponName)) Count))))

(event Custom|Hit
  (bind _targetactor (Variables|TurretInfo|GetTargetActor))
  ;[1 1 1] Call Hit in ShipShieldsSystem
  (Utilities|IsValid _targetactor
    (:Is%20Valid
      (Utilities|Casting|CastToShipBase _targetactor))))

(event Custom|StartCooldownTimer
  ;[1 1 1] Start the cooldown timer for RateOfFire time
  (bind _returnvalue (Utilities|Time|SetTimerbyEvent (delegate Custom|FireTurret) (Variables|TurretInfo|GetRateOfFire))))

(event Custom|FireTurret
  (bind _targetactor (Variables|TurretInfo|GetTargetActor))
  ;[1 1 1] If distance from turret to target <= turret's max range, fire the turret
  (Utilities|IsValid self
    (:Is%20Valid
      (Utilities|IsValid _targetactor
        (:Is%20Valid
          (if (<= (Math|Vector|VectorLength (- (Transformation|GetActorLocation) (Transformation|GetActorLocation _targetactor))) (Variables|TurretInfo|GetMaxRange))
            (CallFunction|CheckFire)))))))

(event EventBeginPlay)

(event Collision|EventActorBeginOverlap
  (params (OtherActor :type Actor%20Object%20Reference)))

(fn ConstructionScript)

(fn DidHit?
  (return (>= (Math|Float|Truncate (+ (Variables|TurretInfo|GetAccuracy) (Math|Conversions|ToFloat(Integer) (Math|Random|RandomIntegerinRange 1 20)))) (+ 10 1))))