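; Planet actor that circles a Pivot actor to simulate a celestial orbit.
; On BeginPlay it takes its starting distance from the Pivot as the orbit radius.
; Each Tick advances an orbit angle by OrbitSpeed and places it on a flat XY circle around the Pivot's current location, so it follows a moving Pivot.
; The angle ignores the initial placement, and the height snaps to the Pivot's.
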(event Custom|Orbit
  (params (Delta :type Float%20%28single-precision%29))
  (bind _orbitdistance (Variables|Default|GetOrbitDistance))
  (bind _output_get (Variables|Default|SetOrbitTime (+ (Variables|Default|GetOrbitTime) (* (Variables|Default|GetOrbitSpeed) Delta))))
  (Transformation|SetActorLocation (+ (Math|Vector|MakeVector (* _orbitdistance (Math|Trig|Cos(Radians) _output_get)) (* _orbitdistance (Math|Trig|Sin(Radians) _output_get)) 0.0) (Transformation|GetActorLocation (Variables|Default|GetPivot))) false false))

(event EventBeginPlay
  (bind _pivot (Variables|Default|GetPivot))
  (Utilities|IsValid _pivot
    (:Is%20Valid
      (Variables|Default|SetOrbitDistance (Math|Vector|VectorLength (- (Transformation|GetActorLocation) (Transformation|GetActorLocation _pivot)))))))

(event Collision|EventActorBeginOverlap
  (params (OtherActor :type Actor%20Object%20Reference)))

(event EventTick
  (params (DeltaSeconds :type Float%20%28single-precision%29))
  (Utilities|IsValid (Variables|Default|GetPivot)
    (:Is%20Valid
      (CallFunction|Orbit DeltaSeconds))))

(fn ConstructionScript)