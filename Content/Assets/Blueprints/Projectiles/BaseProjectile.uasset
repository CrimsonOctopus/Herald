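; Base projectile fired by a shooter, which either homes in on its target or flies straight, depending on a preset Hit flag.
; Tick moves it manually: hits explode on proximity or overlap with the target or a Planet, while misses are destroyed beyond MaxRange from the shooter.
; Explode can report the AttackRoll to the shooter's WeaponObject, then spawns a scaled emitter and destroys the projectile.
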(event Custom|Explode
  (params (Hit :type Actor%20Object%20Reference))
  (if (Utilities|ClassIsChildOf (Utilities|GetClass Hit) 0)
    _
    (else
      (bind _asweapon_object (Utilities|Casting|CastToWeaponObject (Variables|Default|GetShooter)))
      (Default|Hit _asweapon_object (Variables|Default|GetAttackRoll) Hit)))
  (Variables|Default|SetTargetActor 0)
  (bind _returnvalue (Effects|SpawnEmitteratLocation "/Game/Assets/ParticleSystems/ExplosionEffect.ExplosionEffect" (Transformation|GetActorLocation)))
  (Transformation|SetWorldScale3D _returnvalue (Variables|Default|GetExplosionScale))
  (Actor|DestroyActor))

(event EventBeginPlay)

(event Collision|EventActorBeginOverlap
  (params (OtherActor :type Actor%20Object%20Reference))
  (bind _targetactor (Variables|Default|GetTargetActor))
  (if (Variables|Default|GetHit?)
    (Utilities|IsValid _targetactor
      (:Is%20Valid
        (if (== OtherActor _targetactor)
          (CallFunction|Explode _targetactor :!label _label)
          (else
            (if (Utilities|ClassIsChildOf (Utilities|GetClass OtherActor) "/Game/Assets/Blueprints/CelestialObjects/Planet.Planet_C") :!label _label_2
              (goto _label)))))
      (:Is%20Not%20Valid
        (goto _label_2)))))

(event EventTick
  (params (DeltaSeconds :type Float%20%28single-precision%29))
  (Utilities|IsValid (Variables|Default|GetTargetActor)
    (:Is%20Valid
      (if (Variables|Default|GetHit?)
        (bind _directionvector (CallFunction|GetDirectiontoTarget))
        (CallFunction|MoveToward DeltaSeconds _directionvector (Transformation|GetActorLocation (Variables|Default|GetTargetActor)))
        (bind _collided (CallFunction|IsTargetWithinDistance? 5.0))
        (if _collided
          (CallFunction|Explode (Variables|Default|GetTargetActor)))
        (else
          (CallFunction|MoveToward DeltaSeconds (Variables|Default|GetInitialDirection) (Transformation|GetActorForwardVector) :!label _label)
          (bind _collided_2 (CallFunction|IsShooterWithinDistance? (Variables|Default|GetMaxRange)))
          (if (not _collided_2)
            (Actor|DestroyActor)))))
    (:Is%20Not%20Valid
      (goto _label))))

(fn ConstructionScript)

(fn GetDirectiontoTarget
  (return (Math|Vector|Normalize (- (Transformation|GetActorLocation (Variables|Default|GetTargetActor)) (Transformation|GetActorLocation)))))

(fn MoveToward
  (params (DeltaSeconds :type Float%20%28single-precision%29) (MoveDirection :type Vector) (LookTarget :type Vector))
  (bind _newrotation (CallFunction|RotationToward LookTarget))
  (Transformation|SetActorLocationAndRotation (+ (* MoveDirection (* DeltaSeconds (Variables|Default|GetSpeed))) (Transformation|GetActorLocation)) _newrotation))

(fn RotationToward
  (params (Target :type Vector))
  (return (Math|Rotator|FindLookatRotation (Transformation|GetActorLocation) Target)))

(fn IsTargetWithinDistance?
  (params (Distance :type Float%20%28single-precision%29))
  (bind _targetactor (Variables|Default|GetTargetActor))
  (Utilities|IsValid _targetactor
    (:Is%20Valid
      (return (and (Variables|Default|GetHit?) (<= (Math|Vector|VectorLength (- (Transformation|GetActorLocation) (Transformation|GetActorLocation _targetactor))) Distance))))))

(fn IsShooterWithinDistance?
  (params (Distance :type Float%20%28single-precision%29))
  (return (<= (Math|Vector|VectorLength (- (Transformation|GetActorLocation) (Transformation|GetActorLocation (Variables|Default|GetShooter)))) Distance)))